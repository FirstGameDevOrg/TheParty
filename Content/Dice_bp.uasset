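; Dice actor that determines which face is up and stores that value in Points.
; Each Tick, while the static mesh's velocity is exactly zero, NewFunction0 re-evaluates the face.
; It compares the mesh's up, right and forward vectors against world up and down within a tolerance, mapping each match to a face value.
; If none matches, it prints an invalid-dice message and leaves Points unchanged.
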(event `self.ReceiveTick`
  (params (DeltaSeconds :type "Float (single-precision)"))
  (if (== (`KismetMathLibrary.VSize` (`SceneComponent.GetComponentVelocity` (`self.StaticMesh`))) 0.0)
    (`self.NewFunction_0`)))

(fn `NewFunction_0`
  (bind _returnvalue (`SceneComponent.K2_GetComponentRotation` (`self.StaticMesh`)))
  (bind _returnvalue_2 (`KismetMathLibrary.GetUpVector` _returnvalue))
  (bind _returnvalue_3 (`KismetMathLibrary.GetRightVector` _returnvalue))
  (bind _returnvalue_4 (`KismetMathLibrary.GetForwardVector` _returnvalue))
  (if (== _returnvalue_2 (0.0 0.0 1.0) :`ErrorTolerance` 0.1)
    (set `self.points` 6)
    (elif (== _returnvalue_2 (0.0 0.0 -1.0) :`ErrorTolerance` 0.1)
      (set `self.points` 4)
      (elif (== _returnvalue_3 (0.0 0.0 1.0) :`ErrorTolerance` 0.1)
        (set `self.points` 1)
        (elif (== _returnvalue_3 (0.0 0.0 -1.0) :`ErrorTolerance` 0.1)
          (set `self.points` 2)
          (elif (== _returnvalue_4 (0.0 0.0 1.0) :`ErrorTolerance` 0.1)
            (set `self.points` 5)
            (elif (== _returnvalue_4 (0.0 0.0 -1.0) :`ErrorTolerance` 0.1)
              (set `self.points` 3)
              (else
                (`KismetSystemLibrary.PrintString` "骰子不正确")))))))))

(fn `UserConstructionScript`)